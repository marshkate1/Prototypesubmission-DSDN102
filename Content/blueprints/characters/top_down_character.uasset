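; Player character for a Paper2D chameleon game, moving along world Y with jumping, pickups and sprite colour switching on number keys.
; Capsule hits collect bonuses and keys; leaving a level-end overlap shows success or fail widgets based on key count.
; A hitbox repositioned with movement direction enables knockback attacks on enemies, while Tick launches the player during enemy contact and rotates the sprite.
; Colour selection only changes the sprite; vertical movement is disconnected.
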(event OnComponentHit(CapsuleComponent)
  (params (HitComponent :type Primitive%20Component%20Object%20Reference) (OtherActor :type Actor%20Object%20Reference) (OtherComp :type Primitive%20Component%20Object%20Reference) (NormalImpulse :type Vector :default "0, 0, 0") (Hit :type Hit%20Result%20Structure%20%28by%20ref%29))
  (Utilities|FlowControl|Sequence
    (:then_0
      (bind _asbonus (Utilities|Casting|CastTobonus OtherActor))
      (Actor|DestroyActor _asbonus)
      (Variables|Default|Setpoints (+ (Variables|Default|Getpoints) 1)))
    (:then_1
      (bind _askey_1 (Utilities|Casting|CastTokey1 OtherActor))
      (Actor|DestroyActor _askey_1)
      (Variables|Default|Setkeys (+ (Variables|Default|Getkeys) 1) :!label _label))
    (:then_2
      (bind _askey (Utilities|Casting|CastTokey OtherActor))
      (Actor|DestroyActor _askey)
      (goto _label))
    (:then_3
      (bind _askey_2 (Utilities|Casting|CastTokey2 OtherActor))
      (Actor|DestroyActor _askey_2)
      (goto _label))))

(event OnComponentBeginOverlap(overlapbox)
  (params (OverlappedComponent :type Primitive%20Component%20Object%20Reference) (OtherActor :type Actor%20Object%20Reference) (OtherComp :type Primitive%20Component%20Object%20Reference) (OtherBodyIndex :type Integer) (bFromSweep :type Boolean) (SweepResult :type Hit%20Result%20Structure%20%28by%20ref%29))
  (bind _asenemy_v1 (Utilities|Casting|CastToenemy_V1 OtherActor))
  (Variables|Default|Sethit_check_boolean true))

(event OnComponentEndOverlap(overlapbox)
  (params (OverlappedComponent :type Primitive%20Component%20Object%20Reference) (OtherActor :type Actor%20Object%20Reference) (OtherComp :type Primitive%20Component%20Object%20Reference) (OtherBodyIndex :type Integer))
  (bind _returnvalue (Game|GetPlayerController 0))
  (bind _returnvalue_2 (Game|GetPlayerController 0))
  (Utilities|FlowControl|Sequence
    (:then_0
      (Utilities|Casting|CastToenemy_V1 OtherActor)
      (Variables|Default|Sethit_check_boolean false))
    (:then_1
      (Utilities|Casting|CastTolevel_end OtherActor)
      (if (> (Variables|Default|Getkeys) 2)
        (bind _returnvalue_3 (UserInterface|CreateWidget "/Game/blueprints/UI/level_end_success.level_end_success_C"))
        (UserInterface|Viewport|AddtoViewport _returnvalue_3 0)
        (Input|SetInputModeUIOnly _returnvalue _returnvalue_3 "DoNotLock" false)
        (Variables|/Script/Engine.PlayerController|SetbShowMouseCursor _returnvalue true)
        (else
          (bind _returnvalue_4 (UserInterface|CreateWidget "/Game/blueprints/UI/level_end_fail.level_end_fail_C"))
          (UserInterface|Viewport|AddtoViewport _returnvalue_4 0)
          (Input|SetInputModeUIOnly _returnvalue_2 0 "DoNotLock" false)
          (Variables|/Script/Engine.PlayerController|SetbShowMouseCursor _returnvalue_2 true))))))

(event OnComponentBeginOverlap(CapsuleComponent)
  (params (OverlappedComponent :type Primitive%20Component%20Object%20Reference) (OtherActor :type Actor%20Object%20Reference) (OtherComp :type Primitive%20Component%20Object%20Reference) (OtherBodyIndex :type Integer) (bFromSweep :type Boolean) (SweepResult :type Hit%20Result%20Structure%20%28by%20ref%29))
  (Utilities|Casting|CastToenemy_V1 OtherActor)
  (Variables|Default|Setashitplayer true))

(event OnComponentEndOverlap(CapsuleComponent)
  (params (OverlappedComponent :type Primitive%20Component%20Object%20Reference) (OtherActor :type Actor%20Object%20Reference) (OtherComp :type Primitive%20Component%20Object%20Reference) (OtherBodyIndex :type Integer))
  (Utilities|Casting|CastToenemy_V1 OtherActor)
  (Variables|Default|Setashitplayer false))

(event EventBeginPlay
  (bind _returnvalue (UserInterface|CreateWidget "/Game/blueprints/UI/begin_screen.begin_screen_C"))
  (UserInterface|Viewport|AddtoViewport _returnvalue 0)
  (bind _returnvalue_2 (UserInterface|CreateWidget "/Game/blueprints/UI/key_display.key_display_C"))
  (UserInterface|Viewport|AddtoViewport _returnvalue_2 0)
  (bind _returnvalue_3 (UserInterface|CreateWidget "/Game/blueprints/UI/point_display.point_display_C"))
  (UserInterface|Viewport|AddtoViewport _returnvalue_3 0)
  (Utilities|FlowControl|Delay 1.0)
  (bind _asenemy_v1 (Utilities|Casting|CastToenemy_V1 (Game|Player|GetPlayerPawn 0)))
  (bind _output_get (Variables|Default|SetAs%20Enemy%20V1 _asenemy_v1))
  (Development|PrintString (Utilities|String|ToString(Float) (Variables|/Game/blueprints/characters/enemy_V1.enemy_V1_C|Getenemy_forward _output_get))))

(event Collision|EventActorBeginOverlap
  (params (OtherActor :type Actor%20Object%20Reference)))

(event EventTick
  (params (DeltaSeconds :type Float%20%28single-precision%29))
  (bind _keycolour (Variables|Default|GetKeyColour))
  (Utilities|FlowControl|Sequence
    (:then_1
      (if (Variables|Default|Getashitplayer)
        (Character|LaunchCharacter (+ (Variables|/Game/blueprints/characters/enemy_V1.enemy_V1_C|Getenemy_forward (Variables|Default|GetAs%20Enemy%20V1)) "0.000000,-1000.000000,100.000000") false false)))
    (:then_2
      (Math|Float|CompareFloat (.x (Variables|/Script/Engine.MovementComponent|GetVelocity (Variables|Character|GetCharacterMovement))) 0.0
        (:>
          (Transformation|SetRelativeRotation (Variables|Default|GetPaperSprite) "0.000000,-90.000000,0.000000" false false :!label _label))
        (:==
          (if (Variables|Default|Getismovingright)
            (goto _label)
            (else
              (Transformation|SetRelativeRotation (Variables|Default|GetPaperSprite) "0.000000,90.000000,0.000000" false false :!label _label_2))))
        (:<
          (goto _label_2))))
    (:then_3
      (if (not (== _keycolour 0))
        (if (not (== _keycolour 1))
          (if (== _keycolour 2)
            _))))))

(event Input|ActionEvents|InputActionA
  (params (Key :type Key%20Structure :default "None"))
  (:Pressed
    (if (Variables|Default|Gethit_check_boolean)
      (Default|Knockback (stale OnComponentBeginOverlap(overlapbox) _asenemy_v1)))))

(event Input|AxisEvents|InputAxishorizontal
  (params (AxisValue :type Float%20%28single-precision%29))
  (bind _overlapbox (Variables|Default|Getoverlapbox))
  (Pawn|Input|AddMovementInput (Math|Vector|MakeVector 0.0 (Variables|Default|Getspeed) 0.0) AxisValue false)
  (if (> AxisValue 0.0)
    (Transformation|SetRelativeLocation _overlapbox "0.000000,90.000000,0.000000" false false)
    (Variables|Default|Setfoward_vector "0.000000,1.000000,0.000000")
    (Variables|Default|Setismovingright true)
    (elif (< AxisValue 0.0)
      (Transformation|SetRelativeLocation _overlapbox "0.000000,-90.000000,0.000000" false false)
      (Variables|Default|Setfoward_vector "0.000000,-1.000000,0.000000")
      (Variables|Default|Setismovingright false))))

(event Input|AxisEvents|InputAxisvertical
  (params (AxisValue :type Float%20%28single-precision%29)))

(event Input|KeyboardEvents|SpaceBar
  (params (Key :type Key%20Structure :default "None"))
  (:Pressed
    (Character|Jump)))

(event Input|KeyboardEvents|1
  (params (Key :type Key%20Structure :default "None"))
  (:Pressed
    (Variables|Default|SetKeyColour 0)
    (Rendering|Components|Sprite|SetSprite (Variables|Default|GetPaperSprite) "/Game/blueprints/characters/chameleon_Sprite.chameleon_Sprite")))

(event Input|KeyboardEvents|2
  (params (Key :type Key%20Structure :default "None"))
  (:Pressed
    (Variables|Default|SetKeyColour 1)
    (Rendering|Components|Sprite|SetSprite (Variables|Default|GetPaperSprite) "/Game/blueprints/characters/chamaleon_red_sprite.chamaleon_red_sprite")))

(event Input|KeyboardEvents|3
  (params (Key :type Key%20Structure :default "None"))
  (:Pressed
    (Variables|Default|SetKeyColour 2)
    (Rendering|Components|Sprite|SetSprite (Variables|Default|GetPaperSprite) "/Game/blueprints/characters/chamaleon_sprite_blue.chamaleon_sprite_blue")))

(fn ConstructionScript)

(fn PbaFunc
  (Development|PrintString "Hello"))