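; Player character Blueprint that moves along world Y from horizontal input, jumps on SpaceBar and can knock back enemies.
; Horizontal input also shifts Overlapbox to the facing side; its overlaps flag an enemy_V1 for knockback on action A.
; Capsule hits trigger speed pickups, and an event launches the player along X when knocked back.
; Tick prints grounded state from a debug-drawn downward trace; vertical movement logic is disconnected.
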(event OnComponentHit(CapsuleComponent)
  (params (HitComponent :type Primitive%20Component%20Object%20Reference) (OtherActor :type Actor%20Object%20Reference) (OtherComp :type Primitive%20Component%20Object%20Reference) (NormalImpulse :type Vector :default "0, 0, 0") (Hit :type Hit%20Result%20Structure%20%28by%20ref%29))
  (bind _asspeed_pickup (Utilities|Casting|CastTospeed_pickup OtherActor))
  (Default|GivePlayerSpeed _asspeed_pickup)
  (Development|PrintString "yup"))

(event OnComponentBeginOverlap(overlapbox)
  (params (OverlappedComponent :type Primitive%20Component%20Object%20Reference) (OtherActor :type Actor%20Object%20Reference) (OtherComp :type Primitive%20Component%20Object%20Reference) (OtherBodyIndex :type Integer) (bFromSweep :type Boolean) (SweepResult :type Hit%20Result%20Structure%20%28by%20ref%29))
  (bind _asenemy_v1 (Utilities|Casting|CastToenemy_V1 OtherActor))
  (Variables|Default|Sethit_check_boolean true))

(event OnComponentEndOverlap(overlapbox)
  (params (OverlappedComponent :type Primitive%20Component%20Object%20Reference) (OtherActor :type Actor%20Object%20Reference) (OtherComp :type Primitive%20Component%20Object%20Reference) (OtherBodyIndex :type Integer))
  (Utilities|Casting|CastToenemy_V1 OtherActor)
  (Variables|Default|Sethit_check_boolean false))

(event Custom|playerknowckback
  (params (NewParam :type Vector))
  (Character|LaunchCharacter (* NewParam "1000.000000,0.000000,0.000000") false false))

(event EventBeginPlay)

(event Collision|EventActorBeginOverlap
  (params (OtherActor :type Actor%20Object%20Reference)))

(event EventTick
  (params (DeltaSeconds :type Float%20%28single-precision%29))
  (bind _capsulecomponent (Variables|Collision|GetCapsuleComponent))
  (bind _returnvalue (Transformation|GetWorldLocation _capsulecomponent))
  (bind _outhit (Collision|LineTraceByChannel _returnvalue (- _returnvalue "0.000000,0.000000,100.000000") "TraceTypeQuery1" false 0 "Persistent"))
  (if (Actor|ActorHasTag (.HitActor (Collision|BreakHitResult _outhit)) "ground")
    (Development|PrintString "player is grounded")
    (else
      (Development|PrintString "not grounded"))))

(event Input|ActionEvents|InputActionA
  (params (Key :type Key%20Structure :default "None"))
  (:Pressed
    (if (Variables|Default|Gethit_check_boolean)
      (Default|Knockback (stale OnComponentBeginOverlap(overlapbox) _asenemy_v1)))))

(event Input|AxisEvents|InputAxishorizontal
  (params (AxisValue :type Float%20%28single-precision%29))
  (bind _overlapbox (Variables|Default|Getoverlapbox))
  (Pawn|Input|AddMovementInput (Math|Vector|MakeVector 0.0 (Variables|Default|Getspeed) 0.0) AxisValue false)
  (if (> AxisValue 0.0)
    (Transformation|SetRelativeLocation _overlapbox "0.000000,90.000000,0.000000" false false)
    (Variables|Default|Setfoward_vector "0.000000,1.000000,0.000000")
    (elif (< AxisValue 0.0)
      (Transformation|SetRelativeLocation _overlapbox "0.000000,-90.000000,0.000000" false false)
      (Variables|Default|Setfoward_vector "0.000000,-1.000000,0.000000"))))

(event Input|AxisEvents|InputAxisvertical
  (params (AxisValue :type Float%20%28single-precision%29)))

(event Input|KeyboardEvents|SpaceBar
  (params (Key :type Key%20Structure :default "None"))
  (:Pressed
    (Character|Jump)))

(fn ConstructionScript)