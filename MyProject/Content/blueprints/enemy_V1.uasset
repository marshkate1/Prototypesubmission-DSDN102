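; Enemy character for a top-down game that chases the player and trades knockback hits.
; Tick issues AI Move To toward the player pawn unless Stunned.
; Its knockback event stuns it, subtracts the player's Str from Health, then destroys it or launches it using the player's forward vector scaled only on X.
; Capsule hits on the player trigger the player's knockback with the enemy's forward vector, then a timed stun as cooldown.
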(event OnComponentHit(CapsuleComponent)
  (params (HitComponent :type Primitive%20Component%20Object%20Reference) (OtherActor :type Actor%20Object%20Reference) (OtherComp :type Primitive%20Component%20Object%20Reference) (NormalImpulse :type Vector :default "0, 0, 0") (Hit :type Hit%20Result%20Structure%20%28by%20ref%29))
  (bind _astop_down_character (Utilities|Casting|CastTotop_down_character OtherActor))
  (Default|Playerknowckback _astop_down_character (Transformation|GetActorForwardVector))
  (CallFunction|Cooldown))

(event Custom|knockback
  (CallFunction|Stunnedde)
  (bind _astop_down_character (Utilities|Casting|CastTotop_down_character (Game|Player|GetPlayerPawn 0)))
  (Variables|Default|Sethealth (- (Variables|Default|Gethealth) (Variables|/Game/blueprints/top_down_character.top_down_character_C|Getstr _astop_down_character)))
  (if (<= (Variables|Default|Gethealth) 0)
    (Actor|DestroyActor)
    (else
      (Character|LaunchCharacter (* (Variables|/Game/blueprints/top_down_character.top_down_character_C|Getfoward_vector _astop_down_character) "1000.000000,0.000000,0.000000") false false))))

(event Custom|stunnedde
  (Variables|Default|Setstunned true)
  (Components|Movement|StopMovementImmediately (Variables|Character|GetCharacterMovement))
  (Utilities|FlowControl|Delay 2.0)
  (Variables|Default|Setstunned false))

(event Custom|playerknowckback
  (Character|LaunchCharacter "1000.000000,0.000000,0.000000" false false))

(event Custom|cooldown
  (Variables|Default|Setstunned true)
  (Components|Movement|StopMovementImmediately (Variables|Character|GetCharacterMovement))
  (Utilities|FlowControl|Delay 2.0)
  (Variables|Default|Setstunned false))

(event EventBeginPlay)

(event Collision|EventActorBeginOverlap
  (params (OtherActor :type Actor%20Object%20Reference)))

(event EventTick
  (params (DeltaSeconds :type Float%20%28single-precision%29))
  (if (not (Variables|Default|Getstunned))
    (AI|AIMoveTo self "0, 0, 0" (Game|Player|GetPlayerPawn 0) 5.0 false)))

(fn ConstructionScript)